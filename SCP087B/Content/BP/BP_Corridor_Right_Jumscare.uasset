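; Right-corridor jumpscare actor that reveals three staged scare components when the first-person player character enters its Jumscare trigger.
; The overlap makes Jumscare1, Jumscare2 and Jumscare3 visible in turn, separated by short delays, through nested Sequence nodes that also clear each one's hidden-in-game flag.
; Nothing hides them again or guards against re-triggering.
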(event `self.ReceiveBeginPlay`
  (`parent.ReceiveBeginPlay`))

(event `self.Jumscare.OnComponentBeginOverlap`
  (params (OverlappedComponent :type "PrimitiveComponent Object Reference") (OtherActor :type "Actor Object Reference") (OtherComp :type "PrimitiveComponent Object Reference") (OtherBodyIndex :type Integer) (bFromSweep :type Boolean) (SweepResult :type "HitResult Structure (by ref)"))
  (bind _jumscare1 (`self.Jumscare1`))
  (bind _jumscare2 (`self.Jumscare2`))
  (bind _jumscare3 (`self.Jumscare3`))
  (cast `/Game/FirstPerson/Blueprints/BP_FirstPersonCharacter` OtherActor)
  (`|ExecutionSequence`
    (:`then_0`
      (`SceneComponent.SetVisibility` _jumscare1 true true)
      (`KismetSystemLibrary.Delay` 1.2)
      (`|ExecutionSequence`
        (:`then_0`
          (`SceneComponent.SetVisibility` _jumscare2 true true)
          (`KismetSystemLibrary.Delay` 1.2)
          (`|ExecutionSequence`
            (:`then_0`
              (`SceneComponent.SetVisibility` _jumscare3 true true))
            (:`then_1`
              (`SceneComponent.SetHiddenInGame` _jumscare3 false false))))
        (:`then_1`
          (`SceneComponent.SetHiddenInGame` _jumscare2 false false))))
    (:`then_1`
      (`SceneComponent.SetHiddenInGame` _jumscare1 false false))))

(fn `UserConstructionScript`
  (`parent.UserConstructionScript`))