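; Corridor jumpscare actor that slowly creeps toward the player while it is not hidden.
; Each tick it interpolates toward a point just behind player 0, based on that character's forward vector, and snaps its rotation to face the player.
; A KillSelf event destroys the actor; nothing in this Blueprint calls it or changes the hidden state.
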(event `self.ReceiveTick`
  (params (DeltaSeconds :type "Float (single-precision)"))
  (bind _returnvalue (`GameplayStatics.GetPlayerCharacter` 0))
  (bind _returnvalue_2 (`self.K2_GetActorLocation` _returnvalue))
  (if (not (`self.bHidden`))
    (`self.K2_SetActorLocationAndRotation` (`KismetMathLibrary.VInterpTo` (`self.K2_GetActorLocation`) (+ (* (* (`self.GetActorForwardVector` _returnvalue) -1) 1) _returnvalue_2) DeltaSeconds 0.2) (`KismetMathLibrary.FindLookAtRotation` (`self.K2_GetActorLocation`) _returnvalue_2))))

(event `self.ReceiveBeginPlay`
  (`parent.ReceiveBeginPlay`))

(event `Kill Self`
  (`self.K2_DestroyActor`))

(fn `UserConstructionScript`
  (`parent.UserConstructionScript`))